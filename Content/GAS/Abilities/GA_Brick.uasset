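; GA_Brick is an event-activated gameplay ability built around applying the GE_Brick effect to its owner.
; Activation starts a looping timer and prints a debug message.
; A Spawn event, apparently the timer's callback, applies the effect and prints a float attribute from the first player pawn's ability system component.
; The graph never commits or ends the ability, and never clears the timer.
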(event Custom|Spawn
  (Ability|ApplyGameplayEffectToOwner "/Game/GAS/Effects/GE_Brick.GE_Brick_C")
  (Development|PrintString (Utilities|String|ToString(Float) (.ReturnValue (Ability|Attribute|GetFloatAttributefromAbilitySystemComponent (Ability|GetAbilitySystemComponent (Game|Player|GetPlayerPawn 0)) "(AttributeName=\"Shield\",Attribute=/Script/kartelles.BasicAttributeSet:Shield,AttributeOwner=\"/Script/CoreUObject.Class'/Script/kartelles.BasicAttributeSet'\")")))))

(event Ability|EventActivateAbilityFromEvent
  (params (EventData :type Gameplay%20Event%20Data%20Structure%20%28by%20ref%29))
  (Utilities|Time|SetTimerbyEvent (EventDispatchers|CreateEvent :!event Custom|Spawn) 2.5 true)
  (Development|PrintString "Brick Ability"))