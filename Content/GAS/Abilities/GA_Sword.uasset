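; GA_Sword is a Gameplay Ability that gives its user a sword by spawning a BP_Sword actor.
; It activates from a gameplay event, whose OptionalObject supplies the SceneComponent used as the anchor.
; On authority only, it spawns the sword with the anchor's relative transform and attaches it using KeepRelative rules.
; It then calls EndAbilityState; there is no EndAbility call.
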(event Ability|EventActivateAbilityFromEvent
  (params (EventData :type Gameplay%20Event%20Data%20Structure%20%28by%20ref%29))
  (Ability|HasAuthority
    (:True
      (Development|PrintString "Sword Ability")
      (bind _asscene_component (Utilities|Casting|CastToSceneComponent (.OptionalObject (Utilities|Struct|BreakGameplayEventData EventData))))
      (Variables|Default|SetSwordAnchor _asscene_component)
      (bind _returnvalue (Game|SpawnActorfromClass "/Game/Inventory/Items/Weapons/BP_Sword.BP_Sword_C" (Transformation|GetRelativeTransform (Variables|Default|GetSwordAnchor)) "Undefined" "MultiplyWithRoot" 0 0))
      (Transformation|AttachComponentToComponent _returnvalue (Variables|Default|GetSwordAnchor) "None" "KeepRelative" "KeepRelative" "KeepRelative" true)
      (Class|GameplayAbility|EndAbilityState "None"))))