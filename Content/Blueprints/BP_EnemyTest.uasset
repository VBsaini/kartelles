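; BP_EnemyTest is a test enemy actor that damages the player on overlap through the Gameplay Ability System.
; When the overlapping actor casts to BP_Player, the player's ability system component applies GE_DamagePlayer to itself, so the enemy is not the effect's source.
; Debug prints mark the hit and show a float attribute read back from the player's component, with no attribute visibly specified.
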(event EventBeginPlay
  (|CallParentFunction) ; This node is disabled and will not be called.\nDrag off pins to build functionality.
)

(event Collision|EventActorBeginOverlap
  (params (OtherActor :type Actor%20Object%20Reference))
  (|CallParentFunction OtherActor) ; This node is disabled and will not be called.\nDrag off pins to build functionality.
)

(event EventTick
  (params (DeltaSeconds :type Float%20%28single-precision%29)))

(event EventActorBeginOverlap
  (params (OtherActor :type Actor%20Object%20Reference))
  (bind _asbp_player (Utilities|Casting|CastToBP_Player OtherActor))
  (Development|PrintString "DMG" true true "(R=1.000000,G=0.000000,B=0.028406,A=1.000000)")
  (GameplayEffects|ApplyGameplayEffectToTarget :self (Ability|GetAbilitySystemComponent _asbp_player) :GameplayEffectClass "/Game/GAS/Effects/GE_DamagePlayer.GE_DamagePlayer_C" :Target (Ability|GetAbilitySystemComponent _asbp_player))
  (Development|PrintString (Utilities|String|ToString(Float) (.ReturnValue (Ability|Attribute|GetFloatAttributefromAbilitySystemComponent (Ability|GetAbilitySystemComponent _asbp_player) "(AttributeName=\"Health\",Attribute=/Script/kartelles.BasicAttributeSet:Health,AttributeOwner=\"/Script/CoreUObject.Class'/Script/kartelles.BasicAttributeSet'\")")))))

(fn ConstructionScript
  (|CallParentFunction))