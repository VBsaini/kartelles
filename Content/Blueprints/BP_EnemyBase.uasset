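; BP_EnemyBase is an enemy actor that takes damage from sword overlaps through the Gameplay Ability System.
; On BeginPlay it adds the Enemy tag, links itself to its health widget and caches the player after a two-second delay.
; Overlapping a BP_Sword makes the player's ability system apply GE_Watermelon to the enemy, which is destroyed once Health reaches zero or below.
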(event EventBeginPlay
  (Ability|GameplayEffect|AddLooseGameplayTags self (GameplayTags|MakeGameplayTagContainerfromTag "(TagName=\"Enemy\")"))
  (bind _aswbp_enemy_health (Utilities|Casting|CastToWBP_EnemyHealth (UserInterface|GetUserWidgetObject (Variables|Default|GetHealthWidget))))
  (Default|SetEnemyRef _aswbp_enemy_health self)
  (Utilities|FlowControl|Delay 2.0)
  (bind _asbp_player (Utilities|Casting|CastToBP_Player (Game|Player|GetPlayerPawn 0))
    (:then
      (Variables|Default|SetPlayer _asbp_player))
    (:CastFailed
      (Development|PrintString "Hello"))))

(event Collision|EventActorBeginOverlap
  (params (OtherActor :type Actor%20Object%20Reference))
  (Utilities|Casting|CastToBP_Sword OtherActor
    (:then
      (CallFunction|ApplyDamage))
    (:CastFailed
      (Development|PrintString "not  a sword"))))

(fn ConstructionScript)

(fn ApplyDamage
  (GameplayEffects|ApplyGameplayEffectToTarget :self (Ability|GetAbilitySystemComponent (Variables|Default|GetPlayer)) :GameplayEffectClass "/Game/GAS/Effects/GE_Watermelon.GE_Watermelon_C" :Target (Variables|Default|GetAbilitySystemComponent))
  (if (<= (.currentvalue (Variables|/Script/kartelles.BasicAttributeSet|GetHealth (Variables|Default|GetBasicAttributeSet))) 0.0)
    (Actor|DestroyActor)))