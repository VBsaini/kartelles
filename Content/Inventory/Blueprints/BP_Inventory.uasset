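; BP_Inventory manages a grid-based inventory that holds multi-cell items and shows them in an on-screen widget.
; On BeginPlay it fills a flat array with empty cells, adds the inventory widget to the viewport and caches the player pawn.
; Placing an item calls PlaceItem, then creates an item widget positioned and sized on the canvas by cell size.
; Each placement also calls AddAbility on the player and records the item with its grid position.
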(event EventBeginPlay
  (for _index (range 0 (Math|Float|Truncate (- (* (Variables|Default|GetGridHeight) (Variables|Default|GetGridWidth)) 1.0)))
    (Utilities|Array|Add (Variables|Default|GetGridCells) (Utilities|Struct|MakeST_InventoryCell false -1)))
  (bind _returnvalue (UserInterface|CreateWidget "/Game/Inventory/UI/WBP_Inventory.WBP_Inventory_C"))
  (UserInterface|Viewport|AddtoViewport _returnvalue 0)
  (Variables|Default|SetInventoryWidget _returnvalue)
  (bind _asbp_player (Utilities|Casting|CastToBP_Player (Game|Player|GetPlayerPawn 0)))
  (Variables|Default|SetPlayer _asbp_player))

(fn ConstructionScript)

(fn PlaceIteminInventory
  (params (StartX :type Integer) (StartY :type Integer) (ItemData :type Item%20Data%20Structure))
  (bind _cellsize (Variables|Default|GetCellSize))
  (bind _cellsize_2 (Variables|Default|GetCellSize))
  (bind (_width _height) (Utilities|Struct|BreakItemData ItemData))
  (Class|Inventory|PlaceItem StartX StartY ItemData)
  (CallFunction|CreateWidget StartX StartY ItemData)
  (bind _returnvalue (Class|CanvasPanel|AddChildtoCanvas (Variables|/Game/Inventory/UI/WBP_Inventory.WBP_Inventory_C|GetItemCanvasPanel (Variables|Default|GetInventoryWidget)) (Variables|Default|GetCreatedItem)))
  (Class|CanvasPanelSlot|SetPosition _returnvalue (Math|Vector2D|MakeVector2D (* StartX _cellsize_2) (* _cellsize_2 StartY)))
  (Class|CanvasPanelSlot|SetSize _returnvalue (Math|Vector2D|MakeVector2D (* _width _cellsize) (* _cellsize _height)))
  (Default|AddAbility (Variables|Default|GetPlayer))
  (Utilities|Array|Add (Variables|Default|GetPlacedItems) (Utilities|Struct|MakeST_PlacedItem ItemData StartX StartY))
  (Development|PrintString "Adding Ability" true true "(R=1.000000,G=0.784653,B=0.000000,A=1.000000)")
  (return))

(fn CreateWidget
  (params (StartX :type Integer) (StartY :type Integer) (ItemData :type Item%20Data%20Structure))
  (bind _returnvalue (UserInterface|CreateWidget "/Game/Inventory/UI/WBP_InventoryItem.WBP_InventoryItem_C" (Game|GetPlayerController 0) self))
  (Variables|Default|SetCreatedItem _returnvalue)
  (Variables|/Game/Inventory/UI/WBP_InventoryItem.WBP_InventoryItem_C|SetItemData (Variables|Default|GetCreatedItem) ItemData)
  (Variables|/Game/Inventory/UI/WBP_InventoryItem.WBP_InventoryItem_C|SetPositionX (Variables|Default|GetCreatedItem) StartX)
  (Variables|/Game/Inventory/UI/WBP_InventoryItem.WBP_InventoryItem_C|SetPositionY (Variables|Default|GetCreatedItem) StartY))