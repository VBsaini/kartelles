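; BP_WorldItems is a world item pickup that takes its data from DT_ItemData.
; On BeginPlay it loads the DebugRowName row if set, otherwise a random row, and shows that row's icon through its WBP_Items widget.
; When BP_Player overlaps its sphere, it adds the item data to the player's Bag and destroys itself.
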(event OnComponentBeginOverlap(Sphere)
  (params (OverlappedComponent :type Primitive%20Component%20Object%20Reference) (OtherActor :type Actor%20Object%20Reference) (OtherComp :type Primitive%20Component%20Object%20Reference) (OtherBodyIndex :type Integer) (bFromSweep :type Boolean) (SweepResult :type Hit%20Result%20Structure%20%28by%20ref%29))
  (bind _asbp_player (Utilities|Casting|CastToBP_Player OtherActor))
  (bind _output_get (Variables|Default|SetPlayer _asbp_player))
  (Default|AddItem (Variables|/Game/Blueprints/BP_Player.BP_Player_C|GetBag _output_get) (Variables|Default|GetItemData))
  (Actor|DestroyActor))

(event EventBeginPlay
  (bind _debug_rowname (Variables|Default|GetDebug:RowName))
  (bind _outrownames (DataTable|GetDataTableRowNames "/Game/Inventory/Structure/DT_ItemData.DT_ItemData"))
  (if (!= _debug_rowname "")
    (bind _returnvalue (Utilities|GetDataTableRow "/Game/Inventory/Structure/DT_ItemData.DT_ItemData" _debug_rowname)
      (:then
        (Variables|Default|SetItemData _returnvalue)))
    (else
      (bind _returnvalue_2 (Utilities|GetDataTableRow "/Game/Inventory/Structure/DT_ItemData.DT_ItemData" (.OutItem (Utilities|Array|Random _outrownames)))
        (:then
          (Variables|Default|SetItemData _returnvalue_2)))))
  (bind _aswbp_items (Utilities|Casting|CastToWBP_Items (UserInterface|GetUserWidgetObject (Variables|Default|GetWidget))))
  (Default|UpdateImage _aswbp_items (Utilities|Struct|BreakItemData (Variables|Default|GetItemData))))

(fn ConstructionScript)