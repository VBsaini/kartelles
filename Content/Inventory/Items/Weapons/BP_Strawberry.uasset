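; BP_Strawberry is a weapon actor that automatically damages the enemy nearest the player.
; On BeginPlay it caches the player as BP_Player and starts a looping two-second timer that calls Trace.
; Trace gets the player's nearest enemy, line traces from the weapon to it while ignoring both player and weapon, and calls ApplyDamage on BP_EnemyBase if that enemy is hit.
; Debug prints and trace drawing are left on.
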(event Custom|TraceEvent
  (CallFunction|Trace))

(event EventBeginPlay
  (|CallParentFunction)
  (Development|PrintString "SB Spawned")
  (bind _asbp_player (Utilities|Casting|CastToBP_Player (Game|Player|GetPlayerPawn 0)))
  (Variables|Default|SetPlayer _asbp_player)
  (Utilities|Time|SetTimerbyEvent (delegate Custom|TraceEvent) 2.0 true))

(fn ConstructionScript
  (|CallParentFunction))

(fn Trace
  (bind _player (Variables|Default|GetPlayer))
  (Utilities|IsValid _player
    (:Is%20Valid
      (bind _returnvalue (Default|GetNearestEnemy _player))
      (Development|PrintString "Trace" true true "(R=1.000000,G=0.000000,B=0.923175,A=1.000000)")
      (bind _outhit (Collision|LineTraceForObjects (Transformation|GetActorLocation) (Transformation|GetActorLocation _returnvalue) (Utilities|Array|MakeArray "ObjectTypeQuery7") false (Utilities|Array|MakeArray (Variables|Default|GetPlayer) self) "ForDuration"))
      (if (== (.HitActor (Collision|BreakHitResult _outhit)) _returnvalue)
        (bind _asbp_enemy_base (Utilities|Casting|CastToBP_EnemyBase _returnvalue))
        (Default|ApplyDamage _asbp_enemy_base)))))