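; Watermelon weapon projectile that flies at the enemy nearest the player and deals area damage on impact.
; BeginPlay captures start and target positions once; Tick lerps between them with a sine height offset.
; That offset feeds radians into degree-based Sind, so it rises slightly instead of arcing back down.
; When Radius hits, a sphere overlap applies GE_Sword through GAS to the actors found, then the projectile destroys itself.
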(event OnComponentHit(Radius)
  (params (HitComponent :type Primitive%20Component%20Object%20Reference) (OtherActor :type Actor%20Object%20Reference) (OtherComp :type Primitive%20Component%20Object%20Reference) (NormalImpulse :type Vector :default "0, 0, 0") (Hit :type Hit%20Result%20Structure%20%28by%20ref%29))
  (bind _outactors (Collision|SphereOverlapActors (.location (Transformation|GetActorTransform self)) 5e+02 (Utilities|Array|MakeArray "ObjectTypeQuery7" "ObjectTypeQuery3") 0))
  (for _array_element _outactors
    (GameplayEffects|ApplyGameplayEffectToSelf :self (Ability|GetAbilitySystemComponent _array_element) :GameplayEffectClass "/Game/GAS/Effects/GE_Sword.GE_Sword_C")
    (Development|PrintString "dmg" true true "(R=0.000000,G=1.000000,B=0.180299,A=1.000000)"))
  (Actor|DestroyActor))

(event EventBeginPlay
  (|CallParentFunction)
  (bind _returnvalue (Default|GetNearestEnemy (Variables|Default|GetPlayer)))
  (Development|PrintString (Utilities|GetDisplayName _returnvalue))
  (Variables|Default|SetEndLocation (.location (Transformation|GetActorTransform _returnvalue)))
  (Variables|Default|SetStartLocation (.location (Transformation|GetWorldTransform (Variables|/Game/Blueprints/BP_Player.BP_Player_C|GetAnchor (Variables|Default|GetPlayer))))))

(event EventTick
  (params (DeltaSeconds :type Float%20%28single-precision%29))
  (bind _output_get (Variables|Default|SetElasptedTime (+ DeltaSeconds (Variables|Default|GetElasptedTime))))
  (bind _output_get_2 (Variables|Default|SetZoffset (* (Variables|Default|GetArcHeight) (Math|Trig|Sin(Degrees) (* (Math|Float|Clamp(Float) (/ _output_get (Variables|Default|GetTravelTime))) (Math|Trig|GetPI))))))
  (Transformation|SetActorLocation (Math|Vector|MakeVector (.X (Math|Vector|BreakVector (Math|Vector|Lerp(Vector) (Variables|Default|GetStartLocation) (Variables|Default|GetEndLocation) (Math|Float|Clamp(Float) (/ _output_get (Variables|Default|GetTravelTime)))))) (.Y (Math|Vector|BreakVector (Math|Vector|Lerp(Vector) (Variables|Default|GetStartLocation) (Variables|Default|GetEndLocation) (Math|Float|Clamp(Float) (/ _output_get (Variables|Default|GetTravelTime)))))) (+ (.Z (Math|Vector|BreakVector (Math|Vector|Lerp(Vector) (Variables|Default|GetStartLocation) (Variables|Default|GetEndLocation) (Math|Float|Clamp(Float) (/ _output_get (Variables|Default|GetTravelTime)))))) _output_get_2)) false false))

(fn ConstructionScript
  (|CallParentFunction))