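; BP_Items is a pickup actor that adds an item to the player's inventory when walked over.
; On BeginPlay it loads the Skull row from DT_ItemData and pushes that icon to its WBP_Items widget component.
; When BP_Player overlaps the Sphere, it calls PlaceItem on the player's Inventory at a hard-coded grid position, then destroys itself without checking the result.
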(event OnComponentBeginOverlap(Sphere)
  (params (OverlappedComponent :type Primitive%20Component%20Object%20Reference) (OtherActor :type Actor%20Object%20Reference) (OtherComp :type Primitive%20Component%20Object%20Reference) (OtherBodyIndex :type Integer) (bFromSweep :type Boolean) (SweepResult :type Hit%20Result%20Structure%20%28by%20ref%29))
  (bind _asbp_player (Utilities|Casting|CastToBP_Player OtherActor))
  (Default|PlaceItem (Variables|/Game/Blueprints/BP_Player.BP_Player_C|GetInventory _asbp_player) (Variables|Default|GetItemData) 2 3)
  (Actor|DestroyActor))

(event EventBeginPlay
  (bind _returnvalue (Utilities|GetDataTableRow "/Game/Inventory/Structure/DT_ItemData.DT_ItemData" "Skull")
    (:then
      (bind _output_get (Variables|Default|SetItemData _returnvalue))
      (bind _aswbp_items (Utilities|Casting|CastToWBP_Items (UserInterface|GetUserWidgetObject (Variables|Default|GetWidget))))
      (Default|UpdateImage _aswbp_items (.icon _output_get)))))

(fn ConstructionScript)