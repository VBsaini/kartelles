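; BP_IPR_Brick is an inventory placement rule that decides whether a brick item may be placed at a grid cell.
; CanPlace accepts row 5 outright, otherwise it asks the inventory for the item ID at Y+1 and requires ID 5, so placements stack on that item.
; It checks only the start cell's column, ignores the Item argument, and prints the queried ID for debugging.
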(fn CanPlace
  (params (startX :type Integer) (startY :type Integer) (item :type Item%20Data%20Structure))
  (if (== startY 5)
    (return true)
    (else
      (bind _returnvalue (Class|Inventory|GetCellItemId (Variables|Default|GetInvRef) startX (+ startY 1)))
      (Development|PrintString 0 (Utilities|String|ToString(Integer) _returnvalue))
      (if (== _returnvalue 5)
        (return true)
        (else
          (return false))))))