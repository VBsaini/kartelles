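; BP_Store is the item shop, rolling a selection of items and displaying them in the store widget.
; GenerateItems seeds a random stream from the sum of run seed, round and refresh count, making rolls repeatable, then picks DT_ItemData rows with possible duplicates.
; AddItems turns each into a store-sized WBP_InventoryItem in the widget's ItemBox, linked to the inventory.
; A debug function runs both with fixed inputs.
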(event EventBeginPlay)

(event Collision|EventActorBeginOverlap
  (params (OtherActor :type Actor%20Object%20Reference)))

(event EventTick
  (params (DeltaSeconds :type Float%20%28single-precision%29)))

(fn ConstructionScript)

(fn GenerateItems
  (params (RunSeed :type Integer) (RoundNumber :type Integer) (refreshCount :type Integer))
  (LocalVariables|SetRandomStream (Math|Random|MakeRandomStream (+ RunSeed RoundNumber refreshCount)))
  (Utilities|Array|Clear (Variables|Default|GetItems))
  (for _index (range 0 (Variables|Default|GetNumbersOfItem))
    (bind _outrownames (DataTable|GetDataTableRowNames "/Game/Inventory/Structure/DT_ItemData.DT_ItemData"))
    (bind _returnvalue (Utilities|GetDataTableRow "/Game/Inventory/Structure/DT_ItemData.DT_ItemData" (.OutItem (Utilities|Array|RandomFromStream _outrownames (LocalVariables|GetRandomStream))))
      (:then
        (Utilities|Array|Insert (Variables|Default|GetItems) _returnvalue)))))

(fn AddItems
  (for _array_element (Variables|Default|GetItems)
    (bind _returnvalue (UserInterface|CreateWidget "/Game/Inventory/UI/WBP_InventoryItem.WBP_InventoryItem_C" (Game|GetPlayerController 0) (Variables|Default|GetInventoryRef)))
    (Variables|/Game/Inventory/UI/WBP_InventoryItem.WBP_InventoryItem_C|SetItemData _returnvalue _array_element)
    (bind _returnvalue_2 (Class|HorizontalBox|AddChildtoHorizontalBox (Variables|/Game/Store/WBP_Store.WBP_Store_C|GetItemBox (Variables|Default|GetStoreWidget)) _returnvalue))
    (Layout|GridSlot|SetHorizontalAlignment _returnvalue_2 "HAlign_Fill")
    (Layout|GridSlot|SetVerticalAlignment _returnvalue_2 "VAlign_Fill")
    (Variables|/Game/Inventory/UI/WBP_InventoryItem.WBP_InventoryItem_C|SetItemSource _returnvalue "NewEnumerator0")
    (Default|ResizeforStore _returnvalue)))

(fn Debug:MakeStore
  (CallFunction|GenerateItems 0 1 1)
  (CallFunction|AddItems))