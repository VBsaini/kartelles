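; Test Gameplay Ability for the bond system that applies GE_TEST_bond to player 0's pawn.
; On activation it sets the Bond.Test.2 SetByCaller magnitude to a fixed fraction of one of that pawn's float attributes, then applies the spec through the pawn's Ability System Component.
; It prints debug text and an attribute readout, then calls EndAbilityState rather than EndAbility.
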(event Ability|EventActivateAbility
  (Development|PrintString "ability 2")
  (bind _returnvalue (Spec|MakeSpecHandle(ByClass) "/Game/Bonds/GE_TEST_bond.GE_TEST_bond_C" 0))
  (bind _returnvalue_2 (Ability|GameplayEffect|AssignTagSetbyCallerMagnitude _returnvalue "(TagName=\"Bond.Test.2\")" (* (.ReturnValue (Ability|Attribute|GetFloatAttribute (Game|Player|GetPlayerPawn 0) "(AttributeName=\"BaseAttack\",Attribute=/Script/kartelles.DamageAttributeSet:BaseAttack,AttributeOwner=\"/Script/CoreUObject.Class'/Script/kartelles.DamageAttributeSet'\")")) 0.2)))
  (GameplayEffects|ApplyGameplayEffectSpecToSelf (Ability|GetAbilitySystemComponent (Game|Player|GetPlayerPawn 0)) _returnvalue_2)
  (Development|PrintString (Utilities|String|ToString(Float) (.ReturnValue (Ability|Attribute|GetFloatAttributefromAbilitySystemComponent (Ability|GetAbilitySystemComponent (Game|Player|GetPlayerPawn 0)) "(AttributeName=\"Attack\",Attribute=/Script/kartelles.DamageAttributeSet:Attack,AttributeOwner=\"/Script/CoreUObject.Class'/Script/kartelles.DamageAttributeSet'\")"))))
  (Class|GameplayAbility|EndAbilityState "None"))